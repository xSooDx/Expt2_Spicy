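; BP_FemaleCoworkerNPC is an AI-driven coworker NPC that can be called to follow an actor.
; OnCall runs DoCalled, which toggles IsCalled and alternately sets the Blackboard FollowTarget to the calling actor or clears it.
; OnFlirt, OnSpank and OnPraise are placeholder interaction events that only print debug strings.
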(event EventBeginPlay)

(event Collision|EventActorBeginOverlap
  (params (OtherActor :type Actor%20Object%20Reference)))

(event EventTick
  (params (DeltaSeconds :type Float%20%28single-precision%29)))

(event EventOnCall
  (params (Actor :type Actor%20Object%20Reference))
  (Development|PrintString "called")
  (CallFunction|DoCalled Actor))

(event EventOnFlirt
  (params (Actor :type Actor%20Object%20Reference))
  (Development|PrintString "flirt"))

(event EventOnSpank
  (params (Actor :type Actor%20Object%20Reference))
  (Development|PrintString "spank"))

(event EventOnPraise
  (params (ACtor :type Actor%20Object%20Reference))
  (Development|PrintString "praise"))

(fn ConstructionScript)

(fn DoCalled
  (params (B :type Object%20Object%20Reference))
  (AI|Components|Blackboard|SetValueasObject (Utilities|GetAIBlackboard) (Utilities|Name|MakeLiteralName "FollowTarget") (Utilities|SelectObject 0 B (Variables|Default|GetisCalled)))
  (Variables|Default|SetisCalled (not (Variables|Default|GetisCalled))))